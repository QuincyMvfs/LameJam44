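; Timed projectile bomb that shows a countdown widget, then explodes when its detonation delay ends.
; A sphere trace launches player characters away from the blast and applies radial impulse to other hit components.
; Launched players temporarily lose capsule collision to phase through walls.
; The bomb then hides, spawns an explosion effect and a new BP_Bomb_Interactable at ParentLocation, and destroys itself after the phase window.
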(event `self.ReceiveBeginPlay`
  (bind _aswbp_bomb_timer (cast `/Game/Blueprints/UI/WBP_BombTimer` (`WidgetComponent.GetWidget` (`self.Widget`))))
  (bind _output_get (set `self.BombTimer` _aswbp_bomb_timer))
  (`/Game/Blueprints/UI/WBP_BombTimer.StartTimer` _output_get (`self.DelayTillDetonation`))
  (bind _returnvalue (`KismetSystemLibrary.K2_SetTimerDelegate` (delegate `Explode`) (`self.DelayTillDetonation`)))
  (bind _output_get_2 (set `self.DelayTillDetonationTimer` _returnvalue))
  (`/Game/Blueprints/UI/WBP_BombTimer.SetTimer` (`self.BombTimer`) _output_get_2))

(event `Explode`
  (bind _bomb (`self.Bomb`))
  (bind _returnvalue (`SceneComponent.K2_GetComponentLocation` (`self.Bomb`)))
  (bind (_returnvalue_location _returnvalue_rotation _returnvalue_scale) (`KismetMathLibrary.BreakTransform` (`SceneComponent.K2_GetComponentToWorld` (`self.Bomb`))))
  ;[0.1927 0 0] Blow up Bomb
  ;;[1 1 1] Sphere Cast Explosion
  (`self.DrawDebugShpere`)
  (bind _outhits (`KismetSystemLibrary.SphereTraceMultiForObjects` _returnvalue _returnvalue (`self.ExplosionRadius`) (`self.Object Types`)))
  (for _array_element _outhits
    (bind (_bblockinghit _binitialoverlap _time _distance _location _impactpoint _normal _impactnormal _physmat _hitactor _hitcomponent) (`GameplayStatics.BreakHitResult` _array_element))
    ;;[1 1 1] If its the player, launch them up
    (bind _asbp_third_person_character (cast `/Game/Blueprints/Player/BP_ThirdPersonCharacter` _hitactor)
      (:`then`
        (`Character.LaunchCharacter` _asbp_third_person_character (`self.CalculateExplosionForceOnPlayer` _hitactor) false false)
        ;;[0.5651 0.5198 1] Player Phase through walls
        (bind _output_get (set `self.Capsule Component` (`Character.CapsuleComponent` _asbp_third_person_character)))
        (`PrimitiveComponent.SetCollisionEnabled` _output_get "NoCollision")
        (`/Engine/EditorBlueprintResources/StandardMacros.DoOnce` false
          (:`Completed`
            (`KismetSystemLibrary.Delay` (`self.PhaseDuration`))
            (bind _capsule_component (`self.Capsule Component`)
              (:`then`
                (`PrimitiveComponent.SetCollisionEnabled` _capsule_component "QueryAndPhysics"))
              (:`else`)))))
      (:`CastFailed`
        ;;[0.3438 0.3438 0.3438] If not a player, apply impulse
        (`PhysicsObjectBlueprintLibrary.ApplyRadialImpulse` _hitcomponent (`SceneComponent.K2_GetComponentLocation` (`self.Bomb`)) (`self.ExplosionRadius`) (`self.ExplosionStrength`) "RIF_Constant"))))
  ;;[0 0 0] Spawn Explosion and destroy the bomb
  (`GameplayStatics.SpawnEmitterAtLocation` "/Game/StarterContent/Particles/P_Explosion.P_Explosion" _returnvalue_location _returnvalue_rotation _returnvalue_scale)
  (`PrimitiveComponent.SetSimulatePhysics` _bomb false)
  (`PrimitiveComponent.SetCollisionEnabled` _bomb "NoCollision")
  (`SceneComponent.SetVisibility` _bomb false true)
  (`|SpawnActorFromClass` "/Game/Blueprints/Interactables/BP_Bomb_Interactable.BP_Bomb_Interactable_C" (`KismetMathLibrary.MakeTransform` (`self.ParentLocation`)) "Undefined" "MultiplyWithRoot" null null)
  (`KismetSystemLibrary.Delay` (+ (`self.PhaseDuration`) 1.0))
  (`self.K2_DestroyActor`))

(fn `CalculateExplosionForceOnPlayer`
  (params (Player :type "Actor Object Reference"))
  (returns (ExplosionDirection :type "Vector Structure"))
  (return (* (`KismetMathLibrary.Normal` (- (`self.K2_GetActorLocation` Player) (`self.K2_GetActorLocation` self))) (`self.ExplosionStrength`))))

(fn `DrawDebugShpere`
  (`KismetSystemLibrary.DrawDebugSphere` (`SceneComponent.K2_GetComponentLocation` (`self.Bomb`)) (`self.ExplosionRadius`) 12 (struct :`R` 1.0 :`G` 0.182568 :`A` 1.0) 1.0 0.5))

(fn `UserConstructionScript`
  (bind _projectilemovement (`self.ProjectileMovement`))
  (bind _output_get (set `ProjectileMovementComponent.InitialSpeed` (`self.Initial Speed`) _projectilemovement))
  (set `ProjectileMovementComponent.MaxSpeed` _output_get _projectilemovement))