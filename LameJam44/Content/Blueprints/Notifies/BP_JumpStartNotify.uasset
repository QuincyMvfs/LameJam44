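; BP_JumpStartNotify is an animation notify that plays a jump sound for the third-person character.
; When triggered, it casts the mesh owner to BP_ThirdPersonCharacter and does nothing for other actors.
; It picks a random clip from JumpSFX and plays it at the character mesh location with attenuation, randomizing volume and pitch for variety.
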(fn `Received_Notify`
  (params (MeshComp :type "SkeletalMeshComponent Object Reference") (Animation :type "AnimSequenceBase Object Reference") (EventReference :type "AnimNotifyEventReference Structure (by ref)"))
  (returns (ReturnValue :type Boolean))
  (locals (PlayerMesh :type "SkeletalMeshComponent Object Reference"))
  (bind _asbp_third_person_character (cast `/Game/Blueprints/Player/BP_ThirdPersonCharacter` (`ActorComponent.GetOwner` MeshComp)))
  (set `local.PlayerMesh` (`Character.Mesh` _asbp_third_person_character))
  (`GameplayStatics.PlaySoundAtLocation` (`KismetArrayLibrary.Array_Random` (`self.JumpSFX`)) (`SceneComponent.K2_GetComponentLocation` (`local.PlayerMesh`)) (struct) (`KismetMathLibrary.RandomFloatInRange` 0.5 1.2) (`KismetMathLibrary.RandomFloatInRange` 0.9 1.2) 0.0 (`self.Attenuation Settings`) null null null)
  (return false))