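; Interactable locked door that the third-person character opens and closes if it carries a key or the door is already unlocked.
; The first opening consumes the key, spawns an explosion at the lock, hides lock and chains, and leaves the door unlocked.
; A FlipFlop alternates opening and closing, each driven by a looping timer that steps the pivot's yaw toward its limit.
; Open and close sounds play with randomized volume and pitch.
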(event `self.ReceiveBeginPlay`
  (bind (_endrotation_roll _endrotation_pitch _endrotation_yaw) (`KismetMathLibrary.BreakRotator` (`self.EndRotation`)))
  (bind _output_get (set `self.StartRotation` (`SceneComponent.RelativeRotation` (`self.DoorRotationRoot`))))
  (set `self.EndRotation` (`KismetMathLibrary.MakeRotator` (.roll _output_get) (.pitch _output_get) (- (.yaw _output_get) _endrotation_yaw))))

(event `/Game/Blueprints/Interfaces/BPI_Interactable.Interact`
  (params (InteractingActor :type "Actor Object Reference"))
  (bind (_returnvalue_location _returnvalue_rotation _returnvalue_scale) (`KismetMathLibrary.BreakTransform` (`SceneComponent.K2_GetComponentToWorld` (`self.Lock`))))
  (bind _asbp_third_person_character (cast `/Game/Blueprints/Player/BP_ThirdPersonCharacter` InteractingActor))
  (bind _pickupcomponent (`/Game/Blueprints/Player/BP_ThirdPersonCharacter.PickupComponent` _asbp_third_person_character))
  (if (or (`/Game/Blueprints/Player/Components/BPC_Pickup.HasKey?` _pickupcomponent) (`self.IsUnlocked?`))
    (`/Engine/EditorBlueprintResources/StandardMacros.FlipFlop`
      (:`A`
        (`self.TurnOn`)
        (`/Engine/EditorBlueprintResources/StandardMacros.DoOnce` false
          (:`Completed`
            (`GameplayStatics.SpawnEmitterAtLocation` "/Game/StarterContent/Particles/P_Explosion.P_Explosion" _returnvalue_location _returnvalue_rotation _returnvalue_scale)
            (`SceneComponent.SetHiddenInGame` (`self.Chains`) true false)
            (`SceneComponent.SetHiddenInGame` (`self.Lock`) true false)
            (set `/Game/Blueprints/Player/Components/BPC_Pickup.HasKey?` false _pickupcomponent)
            (set `self.IsUnlocked?` true))))
      (:`B`
        (`self.TurnOff`)))))

(event `TurnOn`
  ;[0.1295 1 0.1096] Open Door
  (`GameplayStatics.PlaySoundAtLocation` "/Game/Audio/Door/SFX_Door_Open_01.SFX_Door_Open_01" (`SceneComponent.K2_GetComponentLocation` (`self.Door`)) (struct) (`KismetMathLibrary.RandomFloatInRange` 0.8 1.2) (`KismetMathLibrary.RandomFloatInRange` 0.9 1.1) 0.0 null null null null)
  (`KismetSystemLibrary.K2_ClearAndInvalidateTimerHandle` (`self.DoorMovingTimer`))
  (bind _returnvalue (`KismetSystemLibrary.K2_SetTimerDelegate` (delegate `TurnOn_Animation`) (`self.DoorUpdateSpeed`) true))
  (set `self.DoorMovingTimer` _returnvalue))

(event `TurnOn_Animation`
  (bind (_endrotation_roll _endrotation_pitch _endrotation_yaw) (`KismetMathLibrary.BreakRotator` (`self.EndRotation`)))
  (bind (_relativerotation_roll _relativerotation_pitch _relativerotation_yaw) (`KismetMathLibrary.BreakRotator` (`SceneComponent.RelativeRotation` (`self.DoorRotationRoot`))))
  (bind (_relativerotation_roll_2 _relativerotation_pitch_2 _relativerotation_yaw_2) (`KismetMathLibrary.BreakRotator` (`SceneComponent.RelativeRotation` (`self.DoorRotationRoot`))))
  ;[0.1295 1 0.1096] Open Door
  (if (<= _relativerotation_yaw _endrotation_yaw)
    (`KismetSystemLibrary.K2_ClearAndInvalidateTimerHandle` (`self.DoorMovingTimer`))
    (else
      (`SceneComponent.K2_SetRelativeRotation` (`self.DoorRotationRoot`) (`KismetMathLibrary.MakeRotator` 0.0 0.0 (- _relativerotation_yaw_2 (`self.DoorMovingSpeed`))) false false))))

(event `TurnOff`
  ;[1 0.2292 0.2292] Close Door
  (`KismetSystemLibrary.K2_ClearAndInvalidateTimerHandle` (`self.DoorMovingTimer`))
  (bind _returnvalue (`KismetSystemLibrary.K2_SetTimerDelegate` (delegate `TurnOff_Animation`) (`self.DoorUpdateSpeed`) true))
  (set `self.DoorMovingTimer` _returnvalue))

(event `TurnOff_Animation`
  (bind (_startrotation_roll _startrotation_pitch _startrotation_yaw) (`KismetMathLibrary.BreakRotator` (`self.StartRotation`)))
  (bind (_relativerotation_roll _relativerotation_pitch _relativerotation_yaw) (`KismetMathLibrary.BreakRotator` (`SceneComponent.RelativeRotation` (`self.DoorRotationRoot`))))
  (bind (_relativerotation_roll_2 _relativerotation_pitch_2 _relativerotation_yaw_2) (`KismetMathLibrary.BreakRotator` (`SceneComponent.RelativeRotation` (`self.DoorRotationRoot`))))
  ;[1 0.2292 0.2292] Close Door
  (if (>= _relativerotation_yaw _startrotation_yaw)
    (`KismetSystemLibrary.K2_ClearAndInvalidateTimerHandle` (`self.DoorMovingTimer`))
    (`GameplayStatics.PlaySoundAtLocation` "/Game/Audio/Door/SFX_Door_Close_01.SFX_Door_Close_01" (`SceneComponent.K2_GetComponentLocation` (`self.Door`)) (struct) (`KismetMathLibrary.RandomFloatInRange` 0.8 1.2) (`KismetMathLibrary.RandomFloatInRange` 0.9 1.1) 0.0 null null null null)
    (else
      (`SceneComponent.K2_SetRelativeRotation` (`self.DoorRotationRoot`) (`KismetMathLibrary.MakeRotator` _relativerotation_roll_2 _relativerotation_pitch_2 (+ _relativerotation_yaw_2 (`self.DoorMovingSpeed`))) false false))))

(fn `UserConstructionScript`)