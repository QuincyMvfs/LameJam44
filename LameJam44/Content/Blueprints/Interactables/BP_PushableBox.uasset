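; BP_PushableBox is a pickupable interactable box that destroys itself after running its parent Interact logic.
; When EnablePushingThrough is set, the construction script makes BoxCollision query-only so it detects overlaps.
; An overlapping BPI_Player actor gets EnableCollisionMessage(false) and a slight downward launch, then has it re-enabled after PhaseDuration.
; The trigger collision then switches off, making the push-through one-shot.
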(event `/Game/Blueprints/Interfaces/BPI_Interactable.Interact`
  (params (InteractingActor :type "Actor Object Reference"))
  (`parent.Interact` InteractingActor)
  (`self.K2_DestroyActor`))

(event `self.BoxCollision.OnComponentBeginOverlap`
  (params (OverlappedComponent :type "PrimitiveComponent Object Reference") (OtherActor :type "Actor Object Reference") (OtherComp :type "PrimitiveComponent Object Reference") (OtherBodyIndex :type Integer) (bFromSweep :type Boolean) (SweepResult :type "HitResult Structure (by ref)"))
  (if (`KismetSystemLibrary.DoesImplementInterface` OtherActor "/Game/Blueprints/Interfaces/BPI_Player.BPI_Player_C")
    (message `/Game/Blueprints/Interfaces/BPI_Player.EnableCollision` OtherActor false)
    (`Character.LaunchCharacter` (cast `Character` OtherActor :!pure true) (0.0 0.0 -1.0) false false)
    (`KismetSystemLibrary.Delay` (`self.PhaseDuration`))
    (message `/Game/Blueprints/Interfaces/BPI_Player.EnableCollision` OtherActor true)
    (`PrimitiveComponent.SetCollisionEnabled` (`self.BoxCollision`) "NoCollision")))

(fn `GetIsPickupable`
  (returns (ReturnValue :type Boolean))
  (return true))

(fn `GetObjectType`
  (returns (ObjectType :type "/Game/Blueprints/Enums/EHeldObjectTypes Enum"))
  (return "NewEnumerator1"))

(fn `UserConstructionScript`
  (`PrimitiveComponent.SetCollisionEnabled` (`self.BoxCollision`) (select `bool` (`self.EnablePushingThrough?`) :`false` "NoCollision" :`true` "QueryOnly" :!type "ECollisionEnabled Enum")))