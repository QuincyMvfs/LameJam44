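; BP_Base_Interactable is a base interactable object with placeholder-style Interact behavior and simple query functions.
; Interact spawns an explosion particle at the mesh's location and rotation, then prints a message naming the interacting actor and itself.
; Getters report it as not pickupable, return a fixed object type enum value and expose the mesh's static mesh.
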(event `/Game/Blueprints/Interfaces/BPI_Interactable.Interact`
  (params (InteractingActor :type "Actor Object Reference"))
  (bind _mesh (`self.Mesh`))
  (`GameplayStatics.SpawnEmitterAtLocation` "/Game/StarterContent/Particles/P_Explosion.P_Explosion" (`SceneComponent.K2_GetComponentLocation` _mesh) (`SceneComponent.K2_GetComponentRotation` _mesh))
  (`KismetSystemLibrary.PrintString` (`KismetStringLibrary.Concat_StrStr` (`KismetSystemLibrary.GetDisplayName` InteractingActor) " Interacted With: " (`KismetSystemLibrary.GetDisplayName` self))))

(fn `GetIsPickupable`
  (returns (ReturnValue :type Boolean))
  (return false))

(fn `GetObjectType`
  (returns (ObjectType :type "/Game/Blueprints/Enums/EHeldObjectTypes Enum"))
  (return "NewEnumerator2"))

(fn `GetStaticMesh`
  (returns (Mesh :type "StaticMesh Object Reference"))
  (return (`StaticMeshComponent.StaticMesh` (`self.Mesh`))))

(fn `UserConstructionScript`)