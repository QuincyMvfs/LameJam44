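; Interactable lever that swings its handle between on and off positions, alternating each time it is interacted with.
; BeginPlay caches the handle's world rotation as the start and its negation as the end.
; A FlipFlop restarts a looping timer that steps the handle's roll toward the target.
; Reaching either limit stops the timer and calls LeverEnabled or LeverDisabled; the turn-off check reads relative rather than world roll.
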(event `self.ReceiveBeginPlay`
  ;[0 0 0] Set Defaults
  (bind _output_get (set `self.StartRotation` (`SceneComponent.K2_GetComponentRotation` (`self.LeverHandleRoot`))))
  (set `self.EndRotation` (* _output_get -1.0)))

(event `TurnOn`
  ;[0.1295 1 0.1096] Turn On Lever
  (`KismetSystemLibrary.K2_ClearAndInvalidateTimerHandle` (`self.LeverMovingTimer`))
  (bind _returnvalue (`KismetSystemLibrary.K2_SetTimerDelegate` (delegate `TurnOn_Animation`) (`self.LeverUpdateSpeed`) true))
  (set `self.LeverMovingTimer` _returnvalue))

(event `TurnOn_Animation`
  (bind _endrotation_roll (`KismetMathLibrary.BreakRotator` (`self.EndRotation`)))
  (bind (_returnvalue_roll _returnvalue_pitch _returnvalue_yaw) (`KismetMathLibrary.BreakRotator` (`SceneComponent.K2_GetComponentRotation` (`self.LeverHandleRoot`))))
  (bind _returnvalue_roll_2 (`KismetMathLibrary.BreakRotator` (`SceneComponent.K2_GetComponentRotation` (`self.LeverHandleRoot`))))
  ;[0.1295 1 0.1096] Turn On Lever
  (if (<= _returnvalue_roll_2 _endrotation_roll)
    (`KismetSystemLibrary.K2_ClearAndInvalidateTimerHandle` (`self.LeverMovingTimer`))
    (`self.LeverEnabled`)
    (else
      (`SceneComponent.K2_SetWorldRotation` (`self.LeverHandleRoot`) (`KismetMathLibrary.MakeRotator` (- _returnvalue_roll (`self.LeverMovingSpeed`)) _returnvalue_pitch _returnvalue_yaw) false false))))

(event `TurnOff`
  ;[1 0.2292 0.2292] Turn Off Lever
  (`KismetSystemLibrary.K2_ClearAndInvalidateTimerHandle` (`self.LeverMovingTimer`))
  (bind _returnvalue (`KismetSystemLibrary.K2_SetTimerDelegate` (delegate `TurnOff_Animation`) (`self.LeverUpdateSpeed`) true))
  (set `self.LeverMovingTimer` _returnvalue))

(event `TurnOff_Animation`
  (bind _startrotation_roll (`KismetMathLibrary.BreakRotator` (`self.StartRotation`)))
  (bind (_returnvalue_roll _returnvalue_pitch _returnvalue_yaw) (`KismetMathLibrary.BreakRotator` (`SceneComponent.K2_GetComponentRotation` (`self.LeverHandleRoot`))))
  (bind _relativerotation_roll (`KismetMathLibrary.BreakRotator` (`SceneComponent.RelativeRotation` (`self.LeverHandleRoot`))))
  ;[1 0.2292 0.2292] Turn Off Lever
  (if (>= _relativerotation_roll _startrotation_roll)
    (`KismetSystemLibrary.K2_ClearAndInvalidateTimerHandle` (`self.LeverMovingTimer`))
    (`self.LeverDisabled`)
    (else
      (`SceneComponent.K2_SetWorldRotation` (`self.LeverHandleRoot`) (`KismetMathLibrary.MakeRotator` (+ _returnvalue_roll (`self.LeverMovingSpeed`)) _returnvalue_pitch _returnvalue_yaw) false false))))

(event `/Game/Blueprints/Interfaces/BPI_Interactable.Interact`
  (params (InteractingActor :type "Actor Object Reference"))
  ;[0.8357 0.4913 1] Enable/ Disable Lever
  (`parent.Interact` InteractingActor)
  (`/Engine/EditorBlueprintResources/StandardMacros.FlipFlop`
    (:`A`
      (`self.TurnOn`))
    (:`B`
      (`self.TurnOff`))))

(fn `UserConstructionScript`
  (`parent.UserConstructionScript`))