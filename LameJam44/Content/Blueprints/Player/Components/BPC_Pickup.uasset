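; Player component that lets the third-person character pick up, drop and throw interactable objects (bomb, box, key) and use keys on doors.
; Interacting scans the interaction sphere for BPI_Interactable actors, copies the mesh onto the held-item component and positions it per type.
; Dropping respawns the matching actor, while throwing spawns only bombs, with an initial speed.
; The HasObject RepNotify switches movement state and clears the held mesh.
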(event `self.ReceiveBeginPlay`
  (bind _asbp_third_person_character (cast `/Game/Blueprints/Player/BP_ThirdPersonCharacter` (`self.GetOwner`)))
  (set `self.PlayerRef` _asbp_third_person_character))

(event `AttemptInteract`
  (bind _playerref (`self.PlayerRef`))
  (bind _pickedupitem (`/Game/Blueprints/Player/BP_ThirdPersonCharacter.PickedUpItem` _playerref))
  ;[0.6727 1 0.4651] Interact with object
  (if (not (`self.HasObject`))
    (for _array_element (`PrimitiveComponent.GetOverlappingActors` (`/Game/Blueprints/Player/BP_ThirdPersonCharacter.InteractionSphere` (`self.PlayerRef`)) "/Game/Blueprints/Interactables/BP_Base_Interactable.BP_Base_Interactable_C") :!label _label
      (if (`KismetSystemLibrary.DoesImplementInterface` _array_element "/Game/Blueprints/Interfaces/BPI_Interactable.BPI_Interactable_C")
        (`self.BreakLoop`)
        (set `self.InteracteeInitialLocation` (`Actor.K2_GetActorLocation` _array_element))
        (bind _mesh (message `/Game/Blueprints/Interfaces/BPI_Interactable.GetStaticMesh` _array_element))
        (`StaticMeshComponent.SetStaticMesh` (`/Game/Blueprints/Player/BP_ThirdPersonCharacter.PickedUpItem` (`self.PlayerRef`)) _mesh)
        (bind _returnvalue (message `/Game/Blueprints/Interfaces/BPI_Interactable.GetIsPickupable` _array_element))
        (set `self.HasObject` _returnvalue)
        (bind _objecttype (message `/Game/Blueprints/Interfaces/BPI_Interactable.GetObjectType` _array_element))
        (bind _output_get (set `self.HeldObject` _objecttype))
        (message `/Game/Blueprints/Interfaces/BPI_Interactable.Interact` _array_element (`self.GetOwner`))
        ;[1 1 1] Change Animation item position
        (switch `/Game/Blueprints/Enums/EHeldObjectTypes` _output_get
          (:`NewEnumerator0`
            (`SceneComponent.K2_SetRelativeTransform` _pickedupitem (`/Game/Blueprints/Player/BP_ThirdPersonCharacter.BombTrans` _playerref) false false))
          (:`NewEnumerator1`
            (`SceneComponent.K2_SetRelativeTransform` _pickedupitem (`/Game/Blueprints/Player/BP_ThirdPersonCharacter.BoxTrans` _playerref) false false))
          (:`NewEnumerator3`
            (`SceneComponent.K2_SetRelativeTransform` _pickedupitem (`/Game/Blueprints/Player/BP_ThirdPersonCharacter.KeyTrans` _playerref) false false)))))
    (elif (`self.HasKey?`)
      (`self.SearchForDoor`))))

(event `BreakLoop`
  ;[0.6727 1 0.4651] Interact with object
  (goto _label :!via `Break`))

(event `AttemptDropObject`
  ;[0 0 0] Dropping
  (if (`self.HasObject`)
    (switch `/Game/Blueprints/Enums/EHeldObjectTypes` (`self.HeldObject`)
      (:`NewEnumerator0`
        (`|SpawnActorFromClass` "/Game/Blueprints/LevelElements/BP_ExplodingBomb.BP_ExplodingBomb_C" (`KismetMathLibrary.MakeTransform` (`self.GetSpawnPositionInfront` false) (`Actor.K2_GetActorRotation` (`self.GetOwner`))) "Undefined" "MultiplyWithRoot" null 0.0 (`self.InteracteeInitialLocation`) null)
        (set `self.HasObject` false))
      (:`NewEnumerator1`
        (`|SpawnActorFromClass` "/Game/Blueprints/Interactables/BP_PushableBox.BP_PushableBox_C" (`KismetMathLibrary.MakeTransform` (+ (`Actor.K2_GetActorLocation` (`self.GetOwner`)) (0.0 0.0 200.0))) "Undefined" "MultiplyWithRoot" null true null)
        (set `self.HasObject` false))
      (:`NewEnumerator3`
        (`|SpawnActorFromClass` "/Game/Blueprints/Interactables/BP_Key.BP_Key_C" (`KismetMathLibrary.MakeTransform` (`self.GetSpawnPositionInfront` true)) "Undefined" "MultiplyWithRoot" null null)
        (set `self.HasObject` false)
        (set `self.HasKey?` false)))))

(event `TryThrow`
  (params (`Spawn Transform Location` :type "Vector Structure") (`Spawn Transform Rotation` :type "Rotator Structure") (`Initial Speed` :type "Float (single-precision)"))
  ;[0 0 0] Throw
  (switch `/Game/Blueprints/Enums/EHeldObjectTypes` (`self.HeldObject`)
    (:`NewEnumerator0`
      (`|SpawnActorFromClass` "/Game/Blueprints/LevelElements/BP_ExplodingBomb.BP_ExplodingBomb_C" (`KismetMathLibrary.MakeTransform` `Spawn Transform Location` `Spawn Transform Rotation`) "Undefined" "MultiplyWithRoot" null `Initial Speed` (`self.InteracteeInitialLocation`) null)
      (set `self.HeldObject` "NewEnumerator2")
      (set `self.HasObject` false)
      (set `/Game/Blueprints/Player/BP_ThirdPersonCharacter.MovementState` "NewEnumerator0" (`self.PlayerRef`)))))

(fn `GetSpawnPositionInfront`
  (params (`UseShortRange?` :type Boolean))
  (returns (ReturnValue :type "Vector Structure"))
  (locals (DistanceMultiplier :type "Float (double-precision)"))
  (bind _returnvalue (`self.GetOwner`))
  (if (not `UseShortRange?`)
    (set `local.DistanceMultiplier` (`self.PlaceObjectDistance`))
    (else
      (set `local.DistanceMultiplier` 0.0)))
  (return (+ (`Actor.K2_GetActorLocation` _returnvalue) (* (`Actor.GetActorForwardVector` _returnvalue) (`local.DistanceMultiplier`)))))

(fn `OnRep_HasObject`
  (if (`self.HasObject`)
    (set `/Game/Blueprints/Player/BP_ThirdPersonCharacter.MovementState` "NewEnumerator1" (`self.PlayerRef`))
    (else
      (`StaticMeshComponent.SetStaticMesh` (`/Game/Blueprints/Player/BP_ThirdPersonCharacter.PickedUpItem` (`self.PlayerRef`)) null)
      (set `/Game/Blueprints/Player/BP_ThirdPersonCharacter.MovementState` "NewEnumerator0" (`self.PlayerRef`)))))

(fn `SearchForDoor`
  (for _array_element (`PrimitiveComponent.GetOverlappingActors` (`/Game/Blueprints/Player/BP_ThirdPersonCharacter.InteractionSphere` (`self.PlayerRef`)) "/Game/Blueprints/Interactables/BP_Base_Interactable.BP_Base_Interactable_C")
    (if (`KismetSystemLibrary.DoesImplementInterface` _array_element "/Game/Blueprints/Interfaces/BPI_Interactable.BPI_Interactable_C")
      (cast `/Game/Blueprints/Interactables/BP_Door` _array_element)
      (message `/Game/Blueprints/Interfaces/BPI_Interactable.Interact` _array_element (`self.GetOwner`))
      (set `self.HasObject` false)
      (break))))